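; BP_SubmarinePawn is a player-controlled submarine pawn driven by Enhanced Input move and look actions.
; IA_Move yaws the Box component with its X axis and adds scaled movement input along the actor's forward vector with Y.
; IA_Look adds unclamped relative pitch and yaw to the Camera, with pitch inverted, so looking is separate from steering.
; Input values apply directly without delta-time scaling, and the construction script is empty.
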(event `EnhancedInput|/Game/FirstPerson/Input/Actions/IA_Move`
  (params (ActionValue :type "Vector2D Structure") (ElapsedSeconds :type "Float (double-precision)") (TriggeredSeconds :type "Float (double-precision)") (InputAction :type "InputAction Object Reference" :default "/Game/FirstPerson/Input/Actions/IA_Move.IA_Move"))
  (:`Triggered`
    (`SceneComponent.K2_AddWorldRotation` (`self.Box`) (`KismetMathLibrary.MakeRotator` 0.0 0.0 (/ ActionValue_X 10.0)) false false)
    (`self.AddMovementInput` self (`self.GetActorForwardVector`) (/ ActionValue_Y 5.0) false)))

(event `EnhancedInput|/Game/FirstPerson/Input/Actions/IA_Look`
  (params (ActionValue :type "Vector2D Structure") (ElapsedSeconds :type "Float (double-precision)") (TriggeredSeconds :type "Float (double-precision)") (InputAction :type "InputAction Object Reference" :default "/Game/FirstPerson/Input/Actions/IA_Look.IA_Look"))
  (:`Triggered`
    (`SceneComponent.K2_AddRelativeRotation` (`self.Camera`) (`KismetMathLibrary.MakeRotator` 0.0 (* ActionValue_Y -1.0) ActionValue_X) false false)))

(fn `UserConstructionScript`)