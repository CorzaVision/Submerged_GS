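; BP_GM_MainGame is the main game's Game Mode, tracking connected players and supplying random spawn locations.
; It adds controllers to the AllPlayers array on post-login and controller swap, and removes BP_PC_MainGame controllers on logout.
; FindPlayerStart returns the transform of a randomly chosen PlayerStart, with no occupancy check.
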(event `self.K2_PostLogin`
  (params (NewPlayer :type "PlayerController Object Reference"))
  ;[0 0 0] Player Connection/Disconnection
  ;;[0.1128 0.1128 0.1128] Player Connects Events
  (`KismetArrayLibrary.Array_Add` (`self.All_Players`) NewPlayer))

(event `self.K2_OnSwapPlayerControllers`
  (params (OldPC :type "PlayerController Object Reference") (NewPC :type "PlayerController Object Reference"))
  ;[0 0 0] Player Connection/Disconnection
  ;;[0.1128 0.1128 0.1128] Player Connects Events
  (`KismetArrayLibrary.Array_Add` (`self.All_Players`) NewPC))

(event `self.K2_OnLogout`
  (params (ExitingController :type "Controller Object Reference"))
  ;[0 0 0] Player Connection/Disconnection
  ;;[0.1128 0.1128 0.1128] Player Disconnect Event
  (bind _asbp_pc_main_game (cast `/Game/Submerged/Blueprints/Setup/BP_PC_MainGame` ExitingController))
  (`KismetArrayLibrary.Array_RemoveItem` (`self.All_Players`) _asbp_pc_main_game))

(fn `Find_PlayerStart`
  (returns (Player_Start_Transform :type "Transform Structure (by ref)"))
  (bind _outactors (`GameplayStatics.GetAllActorsOfClass` "/Script/Engine.PlayerStart"))
  (return (`self.GetTransform` (`|GetArrayItem` _outactors (`KismetMathLibrary.RandomIntegerInRange` 0 (- (`KismetArrayLibrary.Array_Length` _outactors) 1))))))

(fn `UserConstructionScript`)