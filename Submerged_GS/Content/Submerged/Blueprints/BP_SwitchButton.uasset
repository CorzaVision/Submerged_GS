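; BP_SwitchButton is an interactable switch that shows or hides a shield Wall.
; On BeginPlay it caches the first actor implementing IA_FPPlayer_Interface, retrying every second until one exists, though nothing here uses that reference afterward.
; Interact waits briefly, then toggles the Wall's visibility using a pair of opposite booleans, ShieldVisible and ShieldInvisible.
; Only visibility changes, without propagating to children; collision is untouched.
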(event `self.ReceiveBeginPlay`
  ;[0 0 0] Get FPPlayer Ref
  (bind _outactors (`GameplayStatics.GetAllActorsWithInterface` "/Game/Submerged/Blueprints/IA_FPPlayer_Interface.IA_FPPlayer_Interface_C" :!label _label))
  (bind _output (`|GetArrayItem` _outactors))
  (`/Engine/EditorBlueprintResources/StandardMacros.IsValid` _output
    (:`Is Valid`
      (set `self.FPRef` _output)
      (`KismetSystemLibrary.PrintString` "Switch Valid"))
    (:`Is Not Valid`
      (`KismetSystemLibrary.Delay` 1.0)
      (goto _label))))

(event `self.Interact`
  (bind _wall (`self.Wall`))
  ;[0 0 0] Send Up Bool
  (`KismetSystemLibrary.Delay` 0.25)
  (if (`self.ShieldVisible`)
    (`SceneComponent.SetVisibility` _wall false false)
    (set `self.ShieldVisible` false)
    (set `self.ShieldInvisible` true)
    (elif (`self.ShieldInvisible`)
      (`SceneComponent.SetVisibility` _wall true false)
      (set `self.ShieldVisible` true)
      (set `self.ShieldInvisible` false))))

(fn `UserConstructionScript`)