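; BP_Sonar is an actor that supplies the player submarine's location and heading to sonar materials through the MP_Sonar parameter collection.
; On BeginPlay it looks up the BP_SubmarineCharacter, retrying every half second until one is valid.
; Each Tick it writes SubPosition with X negated, and SubYaw offset by 90 degrees, adding a full turn when negative.
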(event `self.ReceiveBeginPlay`
  ;[0 0 0] Get Reference to Sub Player
  (bind _outactors (`GameplayStatics.GetAllActorsOfClass` "/Game/Submerged/Blueprints/Characters/BP_SubmarineCharacter.BP_SubmarineCharacter_C" :!label _label))
  (bind _output (`|GetArrayItem` _outactors))
  (`/Engine/EditorBlueprintResources/StandardMacros.IsValid` _output
    (:`Is Valid`
      (set `self.SubCharacter` _output))
    (:`Is Not Valid`
      (`KismetSystemLibrary.Delay` 0.5)
      (goto _label))))

(event `self.ReceiveTick`
  (params (DeltaSeconds :type "Float (single-precision)"))
  (bind _subcharacter (`self.SubCharacter`))
  (bind (_returnvalue_x _returnvalue_y _returnvalue_z) (`KismetMathLibrary.BreakVector` (`self.K2_GetActorLocation` _subcharacter)))
  (bind (_returnvalue_roll _returnvalue_pitch _returnvalue_yaw) (`KismetMathLibrary.BreakRotator` (`self.K2_GetActorRotation` _subcharacter)))
  (bind _returnvalue (+ _returnvalue_yaw 90.0))
  (`/Engine/EditorBlueprintResources/StandardMacros.IsValid` (`self.SubCharacter`)
    (:`Is Valid`
      (`KismetMaterialLibrary.SetVectorParameterValue` "/Game/Submerged/Blueprints/MP_Sonar.MP_Sonar" "SubPosition" (`KismetMathLibrary.Conv_VectorToLinearColor` (`KismetMathLibrary.MakeVector` (* _returnvalue_x -1.0) _returnvalue_y _returnvalue_z)))
      (`KismetMaterialLibrary.SetScalarParameterValue` "/Game/Submerged/Blueprints/MP_Sonar.MP_Sonar" "SubYaw" (`KismetMathLibrary.SelectFloat` (+ _returnvalue 360.0) _returnvalue (< _returnvalue 0.0))))))

(fn `UserConstructionScript`)