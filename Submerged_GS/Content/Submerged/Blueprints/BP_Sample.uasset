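; BP_Sample is a collectible sample in Submerged that the player picks up by interacting with it.
; On BeginPlay it caches a reference to the BP_GS_MainGame game state.
; Its Interact event increments SamplesCollected on that game state, prints the new count and destroys the actor.
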(event `self.ReceiveBeginPlay`
  ;[0 0 0] Get Game State Ref
  (bind _asbp_gs_main_game (cast `/Game/Submerged/Levels/Game/BP_GS_MainGame` (`GameplayStatics.GetGameState`)))
  (set `self.GameStateRef` _asbp_gs_main_game))

(event `/Game/Submerged/Blueprints/Interact_Interface.Interact`
  (bind _gamestateref (`self.GameStateRef`))
  ;[0 0 0] Interact
  (bind _output_get (set `/Game/Submerged/Levels/Game/BP_GS_MainGame.SamplesCollected` (+ (`/Game/Submerged/Levels/Game/BP_GS_MainGame.SamplesCollected` _gamestateref) 1) _gamestateref))
  (`KismetSystemLibrary.PrintString` (`KismetStringLibrary.Conv_IntToString` _output_get))
  (`self.K2_DestroyActor`))

(fn `UserConstructionScript`)