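; Game mode for the main Submerged level that tracks connected player controllers and assigns each a submarine or first-person role.
; PostLogin flags the controller at index 0 as the sub player and otherwise clears the flag on index 1, while swap and logout events update the list.
; SpawnPlayer, not called within this graph, destroys any existing pawn, then spawns and possesses the matching character at a random PlayerStart.
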(event `self.K2_PostLogin`
  (params (NewPlayer :type "PlayerController Object Reference"))
  ;[0 0 0] Player Connection/Disconnection
  ;;[0.1128 0.1128 0.1128] Player Connects Events
  (bind _returnvalue (`KismetArrayLibrary.Array_Add` (`self.All_Players`) NewPlayer))
  (if (== _returnvalue 0)
    (bind _asbp_pc_main_game (cast `/Game/Submerged/Levels/Game/BP_PC_MainGame` (`|GetArrayItem` (`self.All_Players`))))
    (set `/Game/Submerged/Levels/Game/BP_PC_MainGame.Sub_Player` true _asbp_pc_main_game)
    (else
      (bind _asbp_pc_main_game_2 (cast `/Game/Submerged/Levels/Game/BP_PC_MainGame` (`|GetArrayItem` (`self.All_Players`) 1)))
      (set `/Game/Submerged/Levels/Game/BP_PC_MainGame.Sub_Player` false _asbp_pc_main_game_2))))

(event `self.K2_OnSwapPlayerControllers`
  (params (OldPC :type "PlayerController Object Reference") (NewPC :type "PlayerController Object Reference"))
  ;[0 0 0] Player Connection/Disconnection
  ;;[0.1128 0.1128 0.1128] Player Connects Events
  (`KismetArrayLibrary.Array_Add` (`self.All_Players`) NewPC))

(event `self.K2_OnLogout`
  (params (ExitingController :type "Controller Object Reference"))
  ;[0 0 0] Player Connection/Disconnection
  ;;[0.1128 0.1128 0.1128] Player Disconnect Event
  (bind _asbp_pc_main_game (cast `/Game/Submerged/Levels/Game/BP_PC_MainGame` ExitingController))
  (`KismetArrayLibrary.Array_RemoveItem` (`self.All_Players`) _asbp_pc_main_game))

(fn `Find_PlayerStart`
  (returns (Player_Start_Transform :type "Transform Structure (by ref)"))
  (bind _outactors (`GameplayStatics.GetAllActorsOfClass` "/Script/Engine.PlayerStart"))
  (return (`self.GetTransform` (`|GetArrayItem` _outactors (`KismetMathLibrary.RandomIntegerInRange` 0 (- (`KismetArrayLibrary.Array_Length` _outactors) 1))))))

(fn `Spawn_Player`
  (params (Player_Controller :type "PlayerController Object Reference") (Sub_Player :type Boolean))
  (bind _returnvalue (`Controller.K2_GetPawn` Player_Controller))
  (bind _player_start_transform (`self.Find_PlayerStart`))
  (`/Engine/EditorBlueprintResources/StandardMacros.IsValid` _returnvalue
    (:`Is Valid`
      (`self.K2_DestroyActor` _returnvalue))
    (:`Is Not Valid`
      _))
  (if Sub_Player
    (bind _returnvalue_2 (`|SpawnActorFromClass` "/Game/Submerged/Blueprints/Characters/BP_SubmarineCharacter.BP_SubmarineCharacter_C" _player_start_transform "Undefined" "MultiplyWithRoot" null null))
    (`Controller.Possess` Player_Controller _returnvalue_2)
    (else
      (bind _returnvalue_3 (`|SpawnActorFromClass` "/Game/Submerged/Blueprints/Characters/BP_FirstPersonCharacter.BP_FirstPersonCharacter_C" _player_start_transform "Undefined" "MultiplyWithRoot" null null))
      (`Controller.Possess` Player_Controller _returnvalue_3))))

(fn `UserConstructionScript`)