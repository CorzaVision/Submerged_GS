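; Main game mode for Submerged that tracks connected players and provides player spawning.
; PostLogin and controller swaps add controllers to AllPlayers, and logout removes those of type BP_PC_MainGame.
; SpawnPlayer destroys a controller's current pawn, spawns a first-person character at a randomly chosen PlayerStart and possesses it.
; Nothing in this Blueprint calls SpawnPlayer.
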(event `self.K2_PostLogin`
  (params (NewPlayer :type "PlayerController Object Reference"))
  ;[0 0 0] Player Connection/Disconnection
  ;;[0.1128 0.1128 0.1128] Player Connects Events
  (`KismetArrayLibrary.Array_Add` (`self.All_Players`) NewPlayer))

(event `self.K2_OnSwapPlayerControllers`
  (params (OldPC :type "PlayerController Object Reference") (NewPC :type "PlayerController Object Reference"))
  ;[0 0 0] Player Connection/Disconnection
  ;;[0.1128 0.1128 0.1128] Player Connects Events
  (`KismetArrayLibrary.Array_Add` (`self.All_Players`) NewPC))

(event `self.K2_OnLogout`
  (params (ExitingController :type "Controller Object Reference"))
  ;[0 0 0] Player Connection/Disconnection
  ;;[0.1128 0.1128 0.1128] Player Disconnect Event
  (bind _asbp_pc_main_game (cast `/Game/Submerged/Levels/BP_PC_MainGame` ExitingController))
  (`KismetArrayLibrary.Array_RemoveItem` (`self.All_Players`) _asbp_pc_main_game))

(fn `Find_PlayerStart`
  (returns (Player_Start_Transform :type "Transform Structure (by ref)"))
  (bind _outactors (`GameplayStatics.GetAllActorsOfClass` "/Script/Engine.PlayerStart"))
  (return (`self.GetTransform` (`|GetArrayItem` _outactors (`KismetMathLibrary.RandomIntegerInRange` 0 (- (`KismetArrayLibrary.Array_Length` _outactors) 1))))))

(fn `Spawn_Player`
  (params (Player_Controller :type "PlayerController Object Reference"))
  (bind _returnvalue (`Controller.K2_GetPawn` Player_Controller))
  (`/Engine/EditorBlueprintResources/StandardMacros.IsValid` _returnvalue
    (:`Is Valid`
      (`self.K2_DestroyActor` _returnvalue))
    (:`Is Not Valid`
      _))
  (bind _returnvalue_2 (`|SpawnActorFromClass` "/Game/FirstPerson/Blueprints/BP_FirstPersonCharacter.BP_FirstPersonCharacter_C" (`self.Find_PlayerStart`) "Undefined" "MultiplyWithRoot" null null))
  (`Controller.Possess` Player_Controller _returnvalue_2))

(fn `UserConstructionScript`)